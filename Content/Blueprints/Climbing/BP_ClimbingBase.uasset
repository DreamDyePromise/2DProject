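; BP_ClimbingBase is a base climbable object that tells players when they can climb it and when they have reached its top.
; CollisionBox overlaps toggle the player's climb permission, passing this actor as the climb object on entry.
; TopCollisionBox overlaps disable upward climbing at the top and restore it on exit.
; Overlaps are handled only on authority for actors tagged Player, communicating through message calls on the player's reference.
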(event `self.CollisionBox.OnComponentBeginOverlap`
  (params (OverlappedComponent :type "PrimitiveComponent Object Reference") (OtherActor :type "Actor Object Reference") (OtherComp :type "PrimitiveComponent Object Reference") (OtherBodyIndex :type Integer) (bFromSweep :type Boolean) (SweepResult :type "HitResult Structure (by ref)"))
  ;[1 1 1] 攀爬碰撞盒进入或离开时发生的事件
  (`/Engine/EditorBlueprintResources/ActorMacros.Switch Has Authority`
    (:`Authority`
      (if (`self.ActorHasTag` OtherActor "Player")
        (bind _player (message `/Game/Blueprints/Interfaces/INT_PlayerBase.PlayerRef` OtherActor))
        (message `/Game/Blueprints/Interfaces/INT_PlayerBase.CanClimb` _player true self)))))

(event `self.CollisionBox.OnComponentEndOverlap`
  (params (OverlappedComponent :type "PrimitiveComponent Object Reference") (OtherActor :type "Actor Object Reference") (OtherComp :type "PrimitiveComponent Object Reference") (OtherBodyIndex :type Integer))
  ;[1 1 1] 攀爬碰撞盒进入或离开时发生的事件
  (`/Engine/EditorBlueprintResources/ActorMacros.Switch Has Authority`
    (:`Authority`
      (if (`self.ActorHasTag` OtherActor "Player")
        (bind _player (message `/Game/Blueprints/Interfaces/INT_PlayerBase.PlayerRef` OtherActor))
        (message `/Game/Blueprints/Interfaces/INT_PlayerBase.CanClimb` _player false null)))))

(event `self.TopCollisionBox.OnComponentBeginOverlap`
  (params (OverlappedComponent :type "PrimitiveComponent Object Reference") (OtherActor :type "Actor Object Reference") (OtherComp :type "PrimitiveComponent Object Reference") (OtherBodyIndex :type Integer) (bFromSweep :type Boolean) (SweepResult :type "HitResult Structure (by ref)"))
  ;[1 1 1] 当攀爬到顶点的时候不能在往上爬，当在顶点的时候按up键不会触发动画事件
  (`/Engine/EditorBlueprintResources/ActorMacros.Switch Has Authority`
    (:`Authority`
      (if (`self.ActorHasTag` OtherActor "Player")
        (bind _player (message `/Game/Blueprints/Interfaces/INT_PlayerBase.PlayerRef` OtherActor))
        (message `/Game/Blueprints/Interfaces/INT_PlayerBase.SetCanClimbTop` _player false)))))

(event `self.TopCollisionBox.OnComponentEndOverlap`
  (params (OverlappedComponent :type "PrimitiveComponent Object Reference") (OtherActor :type "Actor Object Reference") (OtherComp :type "PrimitiveComponent Object Reference") (OtherBodyIndex :type Integer))
  ;[1 1 1] 当攀爬到顶点的时候不能在往上爬，当在顶点的时候按up键不会触发动画事件
  (`/Engine/EditorBlueprintResources/ActorMacros.Switch Has Authority`
    (:`Authority`
      (if (`self.ActorHasTag` OtherActor "Player")
        (bind _player (message `/Game/Blueprints/Interfaces/INT_PlayerBase.PlayerRef` OtherActor))
        (message `/Game/Blueprints/Interfaces/INT_PlayerBase.SetCanClimbTop` _player true)))))

(fn `UserConstructionScript`)
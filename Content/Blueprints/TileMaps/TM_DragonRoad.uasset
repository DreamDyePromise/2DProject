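; TM_DragonRoad is a tile map Blueprint that pauses a player's camera movement inside its left and right collision boxes.
; On the server, overlaps from actors tagged Player fetch a player reference through a message call.
; That reference is told to pause camera movement on begin overlap and resume it on end overlap, identically for both boxes.
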(event `self.LeftCollisionBox.OnComponentBeginOverlap`
  (params (OverlappedComponent :type "PrimitiveComponent Object Reference") (OtherActor :type "Actor Object Reference") (OtherComp :type "PrimitiveComponent Object Reference") (OtherBodyIndex :type Integer) (bFromSweep :type Boolean) (SweepResult :type "HitResult Structure (by ref)"))
  ;[1 1 1] 客户端or服务端
  (`/Engine/EditorBlueprintResources/ActorMacros.Switch Has Authority`
    (:`Authority`
      (if (`self.ActorHasTag` OtherActor "Player")
        (bind _player (message `/Game/Blueprints/Interfaces/INT_PlayerBase.PlayerRef` OtherActor))
        (message `/Game/Blueprints/Interfaces/INT_PlayerBase.PauseCameraMovement` _player true)))))

(event `self.LeftCollisionBox.OnComponentEndOverlap`
  (params (OverlappedComponent :type "PrimitiveComponent Object Reference") (OtherActor :type "Actor Object Reference") (OtherComp :type "PrimitiveComponent Object Reference") (OtherBodyIndex :type Integer))
  ;[1 1 1] 客户端or服务端
  (`/Engine/EditorBlueprintResources/ActorMacros.Switch Has Authority`
    (:`Authority`
      (if (`self.ActorHasTag` OtherActor "Player")
        (bind _player (message `/Game/Blueprints/Interfaces/INT_PlayerBase.PlayerRef` OtherActor))
        (message `/Game/Blueprints/Interfaces/INT_PlayerBase.PauseCameraMovement` _player false)))))

(event `self.RightCollisionBox.OnComponentBeginOverlap`
  (params (OverlappedComponent :type "PrimitiveComponent Object Reference") (OtherActor :type "Actor Object Reference") (OtherComp :type "PrimitiveComponent Object Reference") (OtherBodyIndex :type Integer) (bFromSweep :type Boolean) (SweepResult :type "HitResult Structure (by ref)"))
  ;[1 1 1] 客户端or服务端
  (`/Engine/EditorBlueprintResources/ActorMacros.Switch Has Authority`
    (:`Authority`
      (if (`self.ActorHasTag` OtherActor "Player")
        (bind _player (message `/Game/Blueprints/Interfaces/INT_PlayerBase.PlayerRef` OtherActor))
        (message `/Game/Blueprints/Interfaces/INT_PlayerBase.PauseCameraMovement` _player true)))))

(event `self.RightCollisionBox.OnComponentEndOverlap`
  (params (OverlappedComponent :type "PrimitiveComponent Object Reference") (OtherActor :type "Actor Object Reference") (OtherComp :type "PrimitiveComponent Object Reference") (OtherBodyIndex :type Integer))
  ;[1 1 1] 客户端or服务端
  (`/Engine/EditorBlueprintResources/ActorMacros.Switch Has Authority`
    (:`Authority`
      (if (`self.ActorHasTag` OtherActor "Player")
        (bind _player (message `/Game/Blueprints/Interfaces/INT_PlayerBase.PlayerRef` OtherActor))
        (message `/Game/Blueprints/Interfaces/INT_PlayerBase.PauseCameraMovement` _player false)))))

(fn `UserConstructionScript`)
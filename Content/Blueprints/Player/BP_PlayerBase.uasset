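; Base multiplayer 2D side-scroller player character with running, jumping, rope/ladder climbing, melee attack, damage and death.
; Input routes through server RPCs that set replicated state, whose OnRep functions update flipbooks, movement mode, collision and position.
; Multicasts play jump sound, knockback and blinking hit effects.
; A spawned BP_Camera follows via timeline lerp toward a timer-sampled player location; pausing that sampling halts the camera at boundaries.
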(event `self.ReceiveBeginPlay`
  ;[1 1 1 1 70] Movement
  (`self.SetPlayerSpawnLocation`)
  ;;[1 1 1] 动态生成BP_Camera，并添加到ViewPoint
  ;;;[1 1 1] 加个延迟，否则后面的运行太快会报空错误，因为可能前面还没生成
  (`KismetSystemLibrary.Delay` 0.05)
  (bind _returnvalue (`|SpawnActorFromClass` "/Game/Blueprints/BP_Camera.BP_Camera_C" (`KismetMathLibrary.MakeTransform` (`self.K2_GetActorLocation`)) "AdjustIfPossibleButAlwaysSpawn" "OverrideRootScale" null null))
  (set `self.PlayerCamera` _returnvalue)
  (bind _playercontroller (message `/Game/Blueprints/Interfaces/INT_PlayerController.PlayerControllerRef` (`self.GetController`)))
  (`/Engine/EditorBlueprintResources/StandardMacros.IsValid` _playercontroller
    (:`Is Valid`
      (`PlayerController.SetViewTargetWithBlend` _playercontroller (`self.PlayerCamera`) 0.0 "VTBlend_Linear" 0.0 false)
      ;;[1 1 1] Camera移动，0.03秒刷一次，同时根据创建的TimeLine曲线来获取对应的数值，将玩家当前位置和Camera的位置进行向量插值运算，设为Camera的新位置
      (`KismetSystemLibrary.K2_SetTimerDelegate` (delegate `UpdatePlayerCameraLocation`) 0.03 true)
      ;;[1 1 1] 防止出现当碰到BoxCollison的时候Camera依旧往后走一段距离，通过在0.2秒调用一下FGetCurrentPlayerLocation方法,这样比camera移动刷新事件的间隔事件0.03秒更久，所以先获取到当前玩家的Location，故当pause的时候设置的是CurrentPlayerLocation，而不会0.03秒刷新
      (bind _returnvalue_2 (`KismetSystemLibrary.K2_SetTimer` null "FGetCurrentPlayerLocation" 0.2 true))
      (set `self.CurrentPlayerLocationHandle` _returnvalue_2))))

(event `UpdatePlayerCameraLocation`
  ;[1 1 1 1 70] Movement
  ;;[1 1 1] Camera移动，0.03秒刷一次，同时根据创建的TimeLine曲线来获取对应的数值，将玩家当前位置和Camera的位置进行向量插值运算，设为Camera的新位置
  (bind (_direction _movementalpha) (`Timeline|PlayerCameraMovement` :!via `PlayFromStart`)
    (:`Update`
      (`self.K2_SetActorLocation` (`self.PlayerCamera`) (`KismetMathLibrary.VLerp` (`self.K2_GetActorLocation` (`self.PlayerCamera`)) (`self.CurrentPlayerLocation`) _movementalpha) false false))))

(event `self.SetPlayerSpawnLocation`
  ;[1 1 1 1 70] Movement
  ;;[1 1 1] 在服务器端获取到Location，保存下来传给客户端使用，防止作弊
  (`self.SRV_SetPlayerSpawnLocation`))

(event `SRV_SetPlayerSpawnLocation`
  ;[1 1 1 1 70] Movement
  ;;[1 1 1] 在服务器端获取到Location，保存下来传给客户端使用，防止作弊
  (bind _gamemode (message `/Game/Blueprints/Interfaces/INT_GameMode.GameModeRef` (`GameplayStatics.GetGameMode`)))
  (set `self.PlayerSpawnLocation` (`/Game/Blueprints/GM_MapleStory.PlayerSpawnLocation` _gamemode)))

(event `self.PauseCameraMovement`
  (params (Pause :type Boolean))
  ;[1 1 1 1 70] Movement
  ;;[1 1 1] Camera移动暂停与否，当Actor碰到两边的BoxCollision
  (`self.CL_PauseCameraMovement` Pause))

(event `CL_PauseCameraMovement`
  (params (Pause :type Boolean))
  (bind _currentplayerlocationhandle (`self.CurrentPlayerLocationHandle`))
  ;[1 1 1 1 70] Movement
  ;;[1 1 1] Camera移动暂停与否，当Actor碰到两边的BoxCollision
  (if Pause
    (`KismetSystemLibrary.K2_PauseTimerHandle` _currentplayerlocationhandle)
    (else
      (`KismetSystemLibrary.K2_UnPauseTimerHandle` _currentplayerlocationhandle))))

(event `InputAxis|Move Left/Right`
  (params (AxisValue :type "Float (single-precision)"))
  (bind (_x _y _z) (`KismetMathLibrary.BreakVector3f` (`self.GetVelocity`)))
  ;[1 1 1 1 70] Movement
  ;;[1 1 1] Player Movement
  (if (and (not (`self.Is Climbing`)) (not (`self.Is Attacking`)) (not (`self.Is Death`)))
    (`self.AddMovementInput` (`KismetMathLibrary.GetForwardVector` (`self.GetControlRotation`)) AxisValue)
    (if (`NavMovementComponent.IsFalling` (`self.CharacterMovement`))
      (if (< _z 0.0)
        (`self.SetMovementState` "NewEnumerator7")
        (elif (> _z 0.0)
          (`self.SetMovementState` "NewEnumerator4")
          (else
            (`self.SetMovementState` "NewEnumerator0"))))
      (elif (< AxisValue 0.0)
        (`self.SetMovementState` "NewEnumerator2")
        (elif (> AxisValue 0.0)
          (`self.SetMovementState` "NewEnumerator1")
          (else
            (`self.SetMovementState` "NewEnumerator0")))))))

(event `InputAxis|Move Up/Down`
  (params (AxisValue :type "Float (single-precision)"))
  (bind _returnvalue_x (`KismetMathLibrary.BreakVector` (`self.K2_GetActorLocation`)))
  ;[1 1 1 1 70] Movement
  ;;[1 1 1] 爬梯子啥的
  (if (and (`self.Is Can Climb`) (not (`self.Is Death`)))
    (`KismetSystemLibrary.PrintString` "Hello")
    (`self.SetZAxisValue` AxisValue)
    (`self.AddMovementInput` (`KismetMathLibrary.GetUpVector` (`self.GetControlRotation`)) AxisValue)
    (if (`self.Is Climbing`)
      (if (and (!= (`self.ZAxis Value`) 0.0) (not (`PaperFlipbookComponent.IsPlaying` (`self.Sprite`))))
        (`self.PauseClimbFlipbook` false)
        (elif (and (== (`self.ZAxis Value`) 0.0) (`PaperFlipbookComponent.IsPlaying` (`self.Sprite`)))
          (`self.PauseClimbFlipbook` true)
          (else
            ;;;[1 1 1 1 10] 判断是否有效，因为一旦离开碰撞体后，会被ClimbObject会被设置为空
            (bind _climb_object (`self.Climb Object`)
              (:`then`
                (bind _returnvalue_x_2 (`KismetMathLibrary.BreakVector` (`self.K2_GetActorLocation` _climb_object)))
                (if (!= _returnvalue_x_2 _returnvalue_x)
                  (`self.AdjustClimbingLocation`)))
              (:`else`))))))))

(event `self.SetZAxisValue`
  (params (ZAxisValue :type "Float (double-precision)"))
  ;[1 1 1 1 70] Movement
  ;;[1 1 1] 爬梯子啥的
  (`self.SRV_SetZAxisValue` ZAxisValue))

(event `SRV_SetZAxisValue`
  (params (ZAxisValue :type "Float (double-precision)"))
  ;[1 1 1 1 70] Movement
  ;;[1 1 1] 爬梯子啥的
  (set `self.ZAxis Value` ZAxisValue))

(event `self.PauseClimbFlipbook`
  (params (bPauseClimbFlipbook :type Boolean))
  ;[1 1 1 1 70] Movement
  ;;[1 1 1] 爬梯子啥的
  (`self.SRV_PauseClimbFlipbook` bPauseClimbFlipbook))

(event `self.AdjustClimbingLocation`
  ;[1 1 1 1 70] Movement
  ;;[1 1 1] 爬梯子啥的
  (`self.SRV_AdjustClimbingLocation`))

(event `SRV_AdjustClimbingLocation`
  (bind (_returnvalue_x _returnvalue_y _returnvalue_z) (`KismetMathLibrary.BreakVector` (`self.K2_GetActorLocation`)))
  ;[1 1 1 1 70] Movement
  ;;[1 1 1] 爬梯子啥的
  (bind _climb_object (`self.Climb Object`)
    (:`then`
      (bind _returnvalue_x_2 (`KismetMathLibrary.BreakVector` (`self.K2_GetActorLocation` _climb_object)))
      ;;;[1 1 1 1 12] 每当设置时就调用附带的回调事件
      (set `self.ClimbingLocation` (`KismetMathLibrary.MakeVector` _returnvalue_x_2 _returnvalue_y _returnvalue_z)))
    (:`else`)))

(event `SRV_PauseClimbFlipbook`
  (params (bPauseClimbFlipbook :type Boolean))
  ;[1 1 1 1 70] Movement
  ;;[1 1 1] 爬梯子啥的
  (set `self.bPauseClimbFlipbook` bPauseClimbFlipbook))

(event `self.SetMovementState`
  (params (MovementState :type "/Game/Blueprints/Enums/E_MovementState Enum" :default "NewEnumerator0"))
  ;[1 1 1 1 70] Movement
  ;;[1 1 1] 封装，使用自定义时间封装代码，防止被随意修改，使其只能够在服务器端被修改
  (`self.SRV_SetMovementState` MovementState))

(event `SRV_SetMovementState`
  (params (MovementState :type "/Game/Blueprints/Enums/E_MovementState Enum" :default "NewEnumerator0"))
  ;[1 1 1 1 70] Movement
  ;;[1 1 1] 封装，使用自定义时间封装代码，防止被随意修改，使其只能够在服务器端被修改
  ;;;[1 1 1] 服务端给客户端返回数据
  (set `self.MovementState` MovementState))

(event `MC_Jump`
  (params (JumpSFX :type "SoundBase Object Reference") (ActorLocation :type "Vector Structure"))
  ;[1 1 1 1 70] Movement
  ;;[1 1 1] 多播，只能在服务器端运行
  (`GameplayStatics.PlaySoundAtLocation` JumpSFX ActorLocation (struct) 1.0 1.0 0.0 null null null null))

(event `InputAction|Jump`
  (params (Key :type "Key Structure"))
  ;[1 1 1 1 70] Movement
  ;;[1 1 1] 跳跃
  (:`Pressed`
    (if (and (`self.FIsNotFalling`) (not (`self.Is Climbing`)) (not (`self.Is Death`)))
      (`self.Jump`)
      (`self.SRV_Jump` (`.JumpSFX_18_A5EC2972447A16B7DE6E27907139B8D6` (break `/Game/Blueprints/Structs/ST_PlayerInfo` (`self.PlayerInfo`))) (`self.K2_GetActorLocation`)))))

(event `SRV_Jump`
  (params (Jump :type "SoundBase Object Reference") (Location :type "Vector Structure"))
  ;[1 1 1 1 70] Movement
  ;;[1 1 1] 多播，只能在服务器端运行
  (`self.MC_Jump` Jump Location))

(event `self.CanClimb`
  (params (bIsCanClimb :type Boolean) (ClimbObject :type "PaperSpriteActor Object Reference"))
  ;[1 1 1 1 70] Movement
  ;;[1 1 1] 攀爬的执行流程判断
  (`self.SRV_CanClimb` bIsCanClimb ClimbObject))

(event `SRV_CanClimb`
  (params (bIsCanClimb :type Boolean) (ClimbObject :type "PaperSpriteActor Object Reference"))
  ;[1 1 1 1 70] Movement
  ;;[1 1 1] 攀爬的执行流程判断
  (set `self.Climb Object` ClimbObject)
  (bind _output_get (set `self.Is Can Climb` bIsCanClimb))
  (if _output_get
    ;;;[1 1 1] 每0.1秒刷新一次，否则除非出碰撞体不然不会在出现overlap事件
    (bind _returnvalue (`KismetSystemLibrary.K2_SetTimerDelegate` (delegate `ClimbInput`) 0.1 true))
    (set `self.CheckClimbInputHandle` _returnvalue)
    (elif (`self.Is Climbing`)
      (`self.SetIsClimbing` false)
      (else
        ;;;[1 1 1] 中止计时，不能攀爬并没有爬
        (`KismetSystemLibrary.K2_ClearAndInvalidateTimerHandle` (`self.CheckClimbInputHandle`))))))

(event `ClimbInput`
  (bind _zaxis_value (`self.ZAxis Value`))
  ;[1 1 1 1 70] Movement
  ;;[1 1 1] 攀爬的执行流程判断
  (if (or (< _zaxis_value 0.0) (and (> _zaxis_value 0.0) (`self.bCanClimbTop`)))
    ;;;[1 1 1] 中止计时，这样就不会老是调用刷新
    (`KismetSystemLibrary.K2_ClearAndInvalidateTimerHandle` (`self.CheckClimbInputHandle`))
    (`self.SetIsClimbing` true)))

(event `self.SetIsClimbing`
  (params (bIsClimbing :type Boolean))
  ;[1 1 1 1 70] Movement
  ;;[1 1 1] 攀爬的执行流程判断
  (`self.SRV_SetIsClimbing` bIsClimbing))

(event `SRV_SetIsClimbing`
  (params (bIsClimbing :type Boolean))
  ;[1 1 1 1 70] Movement
  ;;[1 1 1] 攀爬的执行流程判断
  (set `self.Is Climbing` bIsClimbing))

(event `self.SetCanClimbTop`
  (params (bCanClimbTop :type Boolean))
  ;[1 1 1 1 70] Movement
  ;;[1 1 1] 攀爬的执行流程判断
  (`self.SRV_SetCanClimbTop` bCanClimbTop))

(event `SRV_SetCanClimbTop`
  (params (bCanClimbTop :type Boolean))
  ;[1 1 1 1 70] Movement
  ;;[1 1 1] 攀爬的执行流程判断
  (set `self.bCanClimbTop` bCanClimbTop))

(event `InputAction|Attack`
  (params (Key :type "Key Structure"))
  ;[1 1 1] 攻击敌人
  (:`Pressed`
    (if (and (not (`self.Is Attacking`)) (not (`self.Is Death`)))
      (`self.Attack` true))))

(event `self.Attack`
  (params (bIsAttacking :type Boolean))
  ;[1 1 1] 攻击敌人
  (`self.SRV_Attack` bIsAttacking))

(event `SRV_Attack`
  (params (bIsAttacking :type Boolean))
  (bind _overlappingactors (`self.GetOverlappingActors` "/Game/Blueprints/Enemy/BP_EnemyBase.BP_EnemyBase_C"))
  ;[1 1 1] 攻击敌人
  (set `self.Is Attacking` bIsAttacking)
  (if (!= (`KismetArrayLibrary.Array_Length` _overlappingactors) 0)
    (for _array_element _overlappingactors
      (`GameplayStatics.ApplyDamage` _array_element (* (`.BaseDamage_28_7E5200D44316145824E82EB6C82B4564` (break `/Game/Blueprints/Structs/ST_PlayerInfo` (`self.PlayerInfo`))) (`self.CurrentLevel`)) (`self.GetController`) null "/Script/Engine.DamageType")))
  ;;[1 1 1 1 12] 整个for循环运行结束之后跑，在动画播放完后设置延时在将IsAttacking设为false，这样才不会连续攻击，不延时的话，会出现无法攻击的情况
  (`KismetSystemLibrary.Delay` (`PaperFlipbookComponent.GetFlipbookLength` (`self.Sprite`)))
  (set `self.Is Attacking` false))

(event `self.ReceiveAnyDamage`
  (params (Damage :type "Float (single-precision)") (DamageType :type "DamageType Object Reference") (InstigatedBy :type "Controller Object Reference") (DamageCauser :type "Actor Object Reference"))
  (bind _returnvalue_x (`KismetMathLibrary.BreakVector` (`self.K2_GetActorLocation`)))
  (bind _playerinfo (`self.PlayerInfo`))
  (bind ((`Health_31_7FB48DA140486FA322ACEF9FE4816127` _health)) (break `/Game/Blueprints/Structs/ST_PlayerInfo` _playerinfo))
  (bind _returnvalue_x_2 (`KismetMathLibrary.BreakVector` (`self.K2_GetActorLocation` (`Controller.K2_GetPawn` (`self.EnemyController`)))))
  ;[1 1 1] 被敌人攻击减血
  (set `self.EnemyController` InstigatedBy)
  (set `self.bIsGodMode` true)
  (`self.DamageImpuse` (`KismetMathLibrary.MakeVector` (`KismetMathLibrary.SelectFloat` -350.0 350.0 (< _returnvalue_x _returnvalue_x_2)) 0.0 500.0))
  ;;[1 1 1] 设置受到攻击后玩家的血量
  (bind _structout (setmembers `/Game/Blueprints/Structs/ST_PlayerInfo` :`StructRef` _playerinfo :`Health` (`KismetMathLibrary.FClamp` (- _health Damage) 0.0 _health)))
  (bind _output_get (set `self.PlayerInfo` _structout))
  ;;[1 1 1] 当血量大于0的时候就放受伤效果，小于0就Death
  (if (<= (`.Health_31_7FB48DA140486FA322ACEF9FE4816127` (break `/Game/Blueprints/Structs/ST_PlayerInfo` _output_get)) 0.0)
    (`self.Death` true)
    (else
      (`self.DamageVFX` "/Paper2D/TranslucentUnlitSpriteMaterial.TranslucentUnlitSpriteMaterial" (struct :`R` 1.0 :`G` 1.0 :`B` 1.0 :`A` 0.5))
      (`KismetSystemLibrary.Delay` (`self.GodModeTimer`))
      (set `self.bIsGodMode` false))))

(event `self.DamageVFX`
  (params (PlayerMaterial :type "MaterialInterface Object Reference") (PlayerColor :type "LinearColor Structure"))
  ;[1 1 1] 被敌人攻击后的简单特效
  (`self.SRV_DamageVFX` PlayerMaterial PlayerColor))

(event `self.DamageImpuse`
  (params (Impuse :type "Vector Structure"))
  ;[1 1 1] 被敌人攻击后的简单特效
  (`self.SRV_DamageImpuse` Impuse))

(event `SRV_DamageVFX`
  (params (Material :type "MaterialInterface Object Reference") (Color :type "LinearColor Structure"))
  ;[1 1 1] 被敌人攻击后的简单特效
  (`self.MC_DamageVFX` Material Color))

(event `SRV_DamageImpuse`
  (params (Impuse :type "Vector Structure"))
  ;[1 1 1] 被敌人攻击后的简单特效
  (`self.MC_DamageImpuse` Impuse))

(event `MC_DamageVFX`
  (params (Material :type "MaterialInterface Object Reference") (Color :type "LinearColor Structure"))
  ;[1 1 1] 被敌人攻击后的简单特效
  (bind _returnvalue (`KismetSystemLibrary.K2_SetTimerDelegate` (delegate `DamageVFXLoop`) (/ (`self.GodModeTimer`) 8.0) true))
  (set `self.GodModeTimerHandle` _returnvalue)
  ;;[1 1 1] StopDamageVFX
  (`KismetSystemLibrary.K2_SetTimerDelegate` (delegate `StopDamageVFX`) (`self.GodModeTimer`)))

(event `MC_DamageImpuse`
  (params (Impulse :type "Vector Structure"))
  ;[1 1 1] 被敌人攻击后的简单特效
  (`CharacterMovementComponent.AddImpulse` (`self.CharacterMovement`) Impulse true))

(event `StopDamageVFX`
  ;[1 1 1] 被敌人攻击后的简单特效
  ;;[1 1 1] StopDamageVFX
  (`KismetSystemLibrary.K2_ClearAndInvalidateTimerHandle` (`self.GodModeTimerHandle`)))

(event `DamageVFXLoop`
  (bind _sprite (`self.Sprite`))
  (bind _sprite_2 (`self.Sprite`))
  ;[1 1 1] 被敌人攻击后的简单特效
  (`PrimitiveComponent.SetMaterial` _sprite 0 (stale `MC_DamageVFX` Material))
  (`PaperFlipbookComponent.SetSpriteColor` _sprite (stale `MC_DamageVFX` Color))
  ;;[1 1 1] 恢复原始的Material和颜色
  (`KismetSystemLibrary.Delay` (/ (`self.GodModeTimer`) 16.0))
  (`PrimitiveComponent.SetMaterial` _sprite_2 0 "/Paper2D/MaskedUnlitSpriteMaterial.MaskedUnlitSpriteMaterial")
  (`PaperFlipbookComponent.SetSpriteColor` _sprite_2 (struct :`R` 1.0 :`G` 1.0 :`B` 1.0 :`A` 1.0)))

(event `self.Death`
  (params (bIsDeath :type Boolean))
  ;[1 1 1] Death事件
  (`self.SRV_Death` bIsDeath))

(event `SRV_Death`
  (params (IsDeath :type Boolean))
  ;[1 1 1] Death事件
  (set `self.Is Death` IsDeath))

(fn `FGetCurrentPlayerLocation`
  (set `self.CurrentPlayerLocation` (`self.K2_GetActorLocation`)))

(fn `FIsNotFalling`
  (returns (ReturnValue :type Boolean))
  ;[1 1 1] 未处于掉落状态，即未起跳
  (return (not (`NavMovementComponent.IsFalling` (`self.CharacterMovement`)))))

(fn `OnRep_bPauseClimbFlipbook`
  (bind _sprite (`self.Sprite`))
  (if (`self.bPauseClimbFlipbook`)
    (`PaperFlipbookComponent.Stop` _sprite)
    (else
      (`PaperFlipbookComponent.Play` _sprite))))

(fn `OnRep_ClimbingLocation`
  (`self.K2_SetActorLocation` (`self.ClimbingLocation`)))

(fn `OnRep_Is Attacking`
  (if (`self.Is Attacking`)
    (`self.SetMovementState` "NewEnumerator5")
    (else
      (`self.SetMovementState` "NewEnumerator0"))))

(fn `OnRep_Is Climbing`
  (bind _charactermovement (`self.CharacterMovement`))
  (bind ((`RopeAnimation_22_453465204D1DFB2CFCA65B87874CDC45` _ropeanimation) (`LadderAnimation_21_FEE423314E825C2CFD29B5B7C8F07180` _ladderanimation)) (break `/Game/Blueprints/Structs/ST_PlayerInfo` (`self.PlayerInfo`)))
  (if (`self.Is Climbing`)
    (`CharacterMovementComponent.SetMovementMode` _charactermovement "MOVE_Flying" 0)
    (`PrimitiveComponent.SetCollisionObjectType` (`self.CapsuleComponent`) "ECC_GameTraceChannel1")
    ;[1 1 1] 如果有多种攀爬工具动画，如绳索和梯子，通过这种方法可以使用不同的动画
    (bind _asbp_climbing_base (cast `/Game/Blueprints/Climbing/BP_ClimbingBase` (`self.Climb Object`)))
    (switch `/Game/Blueprints/Enums/E_ClimbingObjectType` (`/Game/Blueprints/Climbing/BP_ClimbingBase.ClimbingObjectType` _asbp_climbing_base)
      (:`NewEnumerator0`
        (`PaperFlipbookComponent.SetFlipbook` (`self.Sprite`) _ropeanimation))
      (:`NewEnumerator1`
        (`PaperFlipbookComponent.SetFlipbook` (`self.Sprite`) _ladderanimation)))
    (else
      (`CharacterMovementComponent.SetMovementMode` _charactermovement "MOVE_Falling" 0)
      (`PrimitiveComponent.SetCollisionObjectType` (`self.CapsuleComponent`) "ECC_Pawn")
      (`PaperFlipbookComponent.SetFlipbook` (`self.Sprite`) (`.JumpAnimation_9_01CC967F4088313CA59CFEA8C33B1269` (break `/Game/Blueprints/Structs/ST_PlayerInfo` (`self.PlayerInfo`)))))))

(fn `OnRep_Is Death`
  (if (`self.Is Death`)
    (`MovementComponent.StopMovementImmediately` (`self.CharacterMovement`))
    (`self.SetMovementState` "NewEnumerator8")))

(fn `OnRep_MovementState`
  (bind _sprite (`self.Sprite`))
  (bind (_idleanimation _runanimation _jumpanimation _fallanimation _stabanimation _ropeanimation _ladderanimation _deadanimation) (break `/Game/Blueprints/Structs/ST_PlayerInfo` (`self.PlayerInfo`)))
  (if (not (`self.Is Climbing`))
    (switch `/Game/Blueprints/Enums/E_MovementState` (`self.MovementState`)
      (:`NewEnumerator0`
        (`PaperFlipbookComponent.SetFlipbook` _sprite _idleanimation))
      (:`NewEnumerator1`
        (`SceneComponent.K2_SetRelativeRotation` :`self` _sprite)
        (`PaperFlipbookComponent.SetFlipbook` _sprite _runanimation))
      (:`NewEnumerator2`
        (`SceneComponent.K2_SetRelativeRotation` _sprite (struct :`Yaw` 180.0) false false)
        (`PaperFlipbookComponent.SetFlipbook` _sprite _runanimation))
      (:`NewEnumerator3`
        (`PaperFlipbookComponent.SetFlipbook` _sprite _ropeanimation))
      (:`NewEnumerator4`
        (`PaperFlipbookComponent.SetFlipbook` _sprite _fallanimation))
      (:`NewEnumerator5`
        (`PaperFlipbookComponent.SetFlipbook` _sprite _stabanimation))
      (:`NewEnumerator7`
        (`PaperFlipbookComponent.SetFlipbook` _sprite _jumpanimation))
      (:`NewEnumerator8`
        (`PaperFlipbookComponent.SetFlipbook` _sprite _deadanimation)))))

(fn `OnRep_PlayerSpawnLocation`
  (`self.K2_SetActorLocation` (`self.PlayerSpawnLocation`)))

(fn `PlayerRef`
  (returns (Player :type "/Game/Blueprints/Player/BP_PlayerBase Object Reference"))
  (return self))

(fn `UserConstructionScript`
  (`parent.UserConstructionScript`))
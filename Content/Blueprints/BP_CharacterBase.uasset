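; BP_CharacterBase is a character base Blueprint that shows floating damage numbers when a player or enemy is hit.
; DisplayFloatingText forwards to an SRV-prefixed event that spawns a BP_FloatingText actor just above the damaged actor.
; A selection picks player or enemy damage, reads the value from that actor's reference getter, and sets a matching color and icon.
; GetCharacterRef returns the character itself.
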(event `/Game/Blueprints/Interfaces/INT_CharacterBase.DisplayFloatingText`
  (params (DamageActor :type "Actor Object Reference") (DisplayFloatingText :type "/Game/Blueprints/Enums/E_FloatingTextType Enum" :default "NewEnumerator0"))
  ;[0 1 0.7422] 当敌人或玩家进行攻击时会漂浮出对应的伤害值以及不同的标签对应不同的受击对象
  (`self.SRV_DisplayFloatText` DamageActor DisplayFloatingText))

(event `SRV_DisplayFloatText`
  (params (DamageActor :type "Actor Object Reference") (Selection :type "/Game/Blueprints/Enums/E_FloatingTextType Enum" :default "NewEnumerator0"))
  ;[0 1 0.7422] 当敌人或玩家进行攻击时会漂浮出对应的伤害值以及不同的标签对应不同的受击对象
  (bind _output_get (set `self.Damage Actor` DamageActor))
  (bind _returnvalue (`|SpawnActorFromClass` "/Game/Blueprints/BP_FloatingText.BP_FloatingText_C" (`KismetMathLibrary.MakeTransform` (`KismetMathLibrary.MakeVector` (.x (`self.K2_GetActorLocation` _output_get)) (.y (`self.K2_GetActorLocation` _output_get)) (+ (.z (`self.K2_GetActorLocation` _output_get)) 30.0))) "Undefined" "OverrideRootScale" null null))
  (bind _output_get_2 (set `self.FloatingText` _returnvalue))
  (switch `/Game/Blueprints/Enums/E_FloatingTextType` Selection
    (:`NewEnumerator0`
      (bind _enemy (message `/Game/Blueprints/Interfaces/INT_EnemyBase.GetEnemyRef` (`self.Damage Actor`)))
      (`/Game/Blueprints/BP_FloatingText.DisplayFloatingText` _output_get_2 (`KismetTextLibrary.Conv_DoubleToText` (`/Game/Blueprints/Enemy/BP_EnemyBase.PlayerDamage` _enemy) "HalfToEven") (struct :`R` 0.464 :`G` 0.678518 :`B` 1.0 :`A` 1.0) "/Game/Assets/UI/Images/IMG_Sword.IMG_Sword"))
    (:`NewEnumerator1`
      (bind _player (message `/Game/Blueprints/Interfaces/INT_PlayerBase.PlayerRef` (`self.Damage Actor`)))
      (`/Game/Blueprints/BP_FloatingText.DisplayFloatingText` _output_get_2 (`KismetTextLibrary.Conv_DoubleToText` (`/Game/Blueprints/Player/BP_PlayerBase.EnemyDamage` _player) "HalfToEven") (struct :`R` 1.0 :`G` 0.479287 :`B` 0.474 :`A` 1.0) "/Game/Assets/UI/Images/IMG_Blood.IMG_Blood"))))

(fn `GetCharacterRef`
  (returns (Character :type "/Game/Blueprints/BP_CharacterBase Object Reference"))
  (return self))

(fn `UserConstructionScript`)
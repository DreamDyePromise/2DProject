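; Base replicated Paper2D enemy that takes hits, chases its attacker, deals contact damage and respawns after death.
; Damage pauses the behavior tree, then loops AIMoveTo around the attacker or, on death, awards experience, fades out and later respawns at a random navmesh point.
; Player overlap toggles a looping server timer that damages non-god-mode players.
; Server events set state, and RepNotifies apply flipbooks, materials, fade color and spawn location.
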(event `/Game/Blueprints/Interfaces/INT_EnemyBase.SetMovementState`
  (params (MovementState :type "/Game/Blueprints/Enums/E_MovementState Enum" :default "NewEnumerator0"))
  (`self.SRV_SetMovementState` MovementState))

(event `SRV_SetMovementState`
  (params (MovementState :type "/Game/Blueprints/Enums/E_MovementState Enum" :default "NewEnumerator0"))
  (set `self.MovementState` MovementState))

(event `self.ReceiveAnyDamage`
  (params (Damage :type "Float (single-precision)") (DamageType :type "DamageType Object Reference") (InstigatedBy :type "Controller Object Reference") (DamageCauser :type "Actor Object Reference"))
  (bind (_returnvalue_x _returnvalue_y _returnvalue_z) (`KismetMathLibrary.BreakVector` (`self.K2_GetActorLocation`)))
  (bind _enemyinfo (`self.EnemyInfo`))
  (bind _enemyinfo_2 (`self.EnemyInfo`))
  (bind ((`HealthBlood_14_32EFAAAC4C2B56585097A09013D44B8F` _healthblood)) (break `/Game/Blueprints/Structs/ST_EnemyInfo` _enemyinfo))
  (bind _returnvalue (`Controller.K2_GetPawn` (`self.PlayerController`)))
  (bind _returnvalue_x_2 (`KismetMathLibrary.BreakVector` (`self.K2_GetActorLocation` (`Controller.K2_GetPawn` (`self.PlayerController`)))))
  ;[0 1 0.2031] 修改Enemy的血量同时设置被攻击后的角色状态
  (set `self.PlayerDamage` Damage)
  (`/Game/Blueprints/Libraries/FunctionLibrary.DisplayFloatingText` self)
  (set `self.PlayerController` InstigatedBy)
  (bind _structout (setmembers `/Game/Blueprints/Structs/ST_EnemyInfo` :`StructRef` _enemyinfo :`HealthBlood` (`KismetMathLibrary.FClamp` (- _healthblood Damage) 0.0 _healthblood)))
  (bind _output_get (set `self.EnemyInfo` _structout))
  (`CharacterMovementComponent.SetMovementMode` (`self.CharacterMovement`) "MOVE_None" 0)
  (`/Game/Blueprints/Interfaces/INT_EnemyBase.SetMovementState` "NewEnumerator9")
  (`BrainComponent.StopLogic` (`AIController.BrainComponent` (`AIBlueprintHelperLibrary.GetAIController` self)) "Hit")
  (`KismetSystemLibrary.Delay` (`PaperFlipbookComponent.GetFlipbookLength` (`self.Sprite`)))
  (if (<= (`.HealthBlood_14_32EFAAAC4C2B56585097A09013D44B8F` (break `/Game/Blueprints/Structs/ST_EnemyInfo` _output_get)) 0.0)
    (bind _player (message `/Game/Blueprints/Interfaces/INT_PlayerBase.PlayerRef` (`Controller.K2_GetPawn` (`self.PlayerController`))))
    (message `/Game/Blueprints/Interfaces/INT_PlayerBase.AddExperience` _player (`.Experience_36_1AA4FC9948042C66FB844697F6AE131B` (break `/Game/Blueprints/Structs/ST_EnemyInfo` (`self.EnemyInfo`))))
    ;[0 0.4375 1] 敌人死亡，首先取消Overlap事件，之后产生Fade效果，然后在一段时间后自动重生，逆着来一遍Fade，重新开启行为树，开启碰撞体的Overlap事件，设置为不死状态
    (`/Game/Blueprints/Interfaces/INT_EnemyBase.Death` true)
    (set `PrimitiveComponent.bGenerateOverlapEvents` false (`self.HitBox`))
    (set `PrimitiveComponent.bGenerateOverlapEvents` false (`self.Collision`))
    (`/Game/Blueprints/Interfaces/INT_EnemyBase.EnemyFade` true)
    (`KismetSystemLibrary.Delay` (`.RespawnTimer_26_878E2D49428FBB8277568C82C851F01C` (break `/Game/Blueprints/Structs/ST_EnemyInfo` (`self.EnemyInfo`))))
    (bind _structout_2 (setmembers `/Game/Blueprints/Structs/ST_EnemyInfo` :`StructRef` _enemyinfo_2 :`HealthBlood` (`.MaxHealth_23_3BC4DA72471ECC49285DB68D2ECD8DD0` (break `/Game/Blueprints/Structs/ST_EnemyInfo` _enemyinfo_2))))
    (set `self.EnemyInfo` _structout_2)
    (set `PrimitiveComponent.bGenerateOverlapEvents` true (`self.Hitbox`))
    (set `PrimitiveComponent.bGenerateOverlapEvents` true (`self.Collision`))
    (`CharacterMovementComponent.SetMovementMode` (`self.CharacterMovement`) "MOVE_Walking" 0)
    (`/Game/Blueprints/Interfaces/INT_EnemyBase.SetMovementState` "NewEnumerator1")
    (`/Game/Blueprints/Interfaces/INT_EnemyBase.Respawn`)
    (`/Game/Blueprints/Interfaces/INT_EnemyBase.EnemyFade` false)
    (`/Game/Blueprints/Interfaces/INT_EnemyBase.RestartBehaviorTree`)
    (else
      ;[0 1 0.4141] 敌人没死
      (`CharacterMovementComponent.SetMovementMode` (`self.CharacterMovement`) "MOVE_Walking" 0)
      (`/Game/Blueprints/Interfaces/INT_EnemyBase.SetMovementState` "NewEnumerator1")
      ;;[0 0.5078 1] Enemy向着攻击自己的玩家追逐，当半径为2个单位的时候表示已经追到
      (`|AIMoveTo` self (`self.K2_GetActorLocation` _returnvalue) _returnvalue 2.0 :!label _label
        (:`OnSuccess`
          ;;[0.3594 1 0] 玩家死亡那么敌人就不在追逐玩家
          (bind _player_2 (message `/Game/Blueprints/Interfaces/INT_PlayerBase.PlayerRef` (`Controller.K2_GetPawn` (`self.PlayerController`))))
          (if (not (`/Game/Blueprints/Player/BP_PlayerBase.Is Death` _player_2))
            ;;[0 0.7656 1] Enemy在Player身前身后125个单位内的范围内反复移动
            (`AITask_MoveTo.AIMoveTo` (`AIBlueprintHelperLibrary.GetAIController` self) (`KismetMathLibrary.MakeVector` (+ (`KismetMathLibrary.SelectFloat` -125.0 125.0 (< _returnvalue_x_2 _returnvalue_x)) _returnvalue_x) _returnvalue_y _returnvalue_z) null
              (:`OnMoveFinished`
                (goto _label)))
            (else
              (`/Game/Blueprints/Interfaces/INT_EnemyBase.RestartBehaviorTree`))))))))

(event `/Game/Blueprints/Interfaces/INT_EnemyBase.StartApplyDamage`
  (params (bApplyDamage :type Boolean))
  ;[0 0.7656 1] 敌人对玩家造成伤害
  (`self.SRV_StartApplyDamage` bApplyDamage))

(event `SRV_StartApplyDamage`
  (params (bApplyDamage :type Boolean))
  ;[0 0.7656 1] 敌人对玩家造成伤害
  ;;[0 0.9766 1 1 10] 设置计时器，当碰撞器一直重叠的时候不会发生只造成一次伤害的情况，而是持续刷新，但是要Apply Damage为false的时候，意味着没有和玩家碰撞体重叠，这是需要报计时器clear，不然ApplyDamage会一直运行，当检测到可以和敌人碰撞体发生交互的物体的时候，就会触发这个ApplyDamage事件，但是clear就说明玩家不在敌人的碰撞体范围内
  (if bApplyDamage
    (bind _returnvalue (`KismetSystemLibrary.K2_SetTimerDelegate` (delegate `ApplyDamage`) 0.1 true))
    (set `self.ApplyDamageHandle` _returnvalue)
    (else
      (`KismetSystemLibrary.K2_ClearAndInvalidateTimerHandle` (`self.ApplyDamageHandle`)))))

(event `ApplyDamage`
  ;[0 0.7656 1] 敌人对玩家造成伤害
  (for _array_element (`self.GetOverlappingActors` "/Game/Blueprints/Player/BP_PlayerBase.BP_PlayerBase_C")
    (bind _player (message `/Game/Blueprints/Interfaces/INT_PlayerBase.PlayerRef` _array_element))
    (if (not (`/Game/Blueprints/Player/BP_PlayerBase.bIsGodMode` _player))
      (`GameplayStatics.ApplyDamage` _array_element (`.Damage_17_8DB059014270C8545D9244A19FE60BB6` (break `/Game/Blueprints/Structs/ST_EnemyInfo` (`self.EnemyInfo`))) (`self.GetController`) null "/Script/Engine.DamageType"))))

(event `self.Collision.OnComponentBeginOverlap`
  (params (OverlappedComponent :type "PrimitiveComponent Object Reference") (OtherActor :type "Actor Object Reference") (OtherComp :type "PrimitiveComponent Object Reference") (OtherBodyIndex :type Integer) (bFromSweep :type Boolean) (SweepResult :type "HitResult Structure (by ref)"))
  ;[0 0.8594 1] Overlap事件，主要是和Player碰撞体进行检测
  (`/Engine/EditorBlueprintResources/ActorMacros.Switch Has Authority`
    (:`Authority`
      (if (`self.ActorHasTag` OtherActor "Player")
        (`/Game/Blueprints/Interfaces/INT_EnemyBase.StartApplyDamage` true)))))

(event `/Game/Blueprints/Interfaces/INT_EnemyBase.Respawn`
  ;[0 0.6016 1] 敌人重生
  (`self.SRV_Respawn`))

(event `/Game/Blueprints/Interfaces/INT_EnemyBase.Death`
  (params (bIsDeath :type Boolean))
  ;[1 0 0.4922] 敌人死亡事件
  (`self.SRV_Death` bIsDeath))

(event `self.Collision.OnComponentEndOverlap`
  (params (OverlappedComponent :type "PrimitiveComponent Object Reference") (OtherActor :type "Actor Object Reference") (OtherComp :type "PrimitiveComponent Object Reference") (OtherBodyIndex :type Integer))
  ;[0 0.8594 1] Overlap事件，主要是和Player碰撞体进行检测
  (`/Engine/EditorBlueprintResources/ActorMacros.Switch Has Authority`
    (:`Authority`
      (if (`self.ActorHasTag` OtherActor "Player")
        (`/Game/Blueprints/Interfaces/INT_EnemyBase.StartApplyDamage` false)))))

(event `SRV_Respawn`
  ;[0 0.6016 1] 敌人重生
  (bind _returnvalue (`GameplayStatics.GetActorOfClass` "/Script/NavigationSystem.NavMeshBoundsVolume"))
  (bind (_x _y _z) (`KismetMathLibrary.BreakVector3f` (`NavigationSystemV1.K2_GetRandomReachablePointInRadius` (`self.K2_GetActorLocation`) (`KismetMathLibrary.BreakVector3f` (`.BoxExtent` (`self.GetActorBounds` _returnvalue false false))) null null)))
  (set `self.SpawnLocation` (`KismetMathLibrary.MakeVector` _x (`.Y` (`KismetMathLibrary.BreakVector3f` (`self.K2_GetActorLocation`))) (+ _z 20.0))))

(event `SRV_Death`
  (params (bIsDeath :type Boolean))
  ;[1 0 0.4922] 敌人死亡事件
  (bind _output_get (set `self.Is Death` bIsDeath))
  (if _output_get
    (`self.MC_DeathSound` (`.DeathSFX_29_325EAEF846CE5C6191C8A29620138D4A` (break `/Game/Blueprints/Structs/ST_EnemyInfo` (`self.EnemyInfo`))) (`self.K2_GetActorLocation`))))

(event `/Game/Blueprints/Interfaces/INT_EnemyBase.RestartBehaviorTree`
  ;[1 0 0.2578] Restart Behavior Tree
  (`self.CL_RestartBehaviorTree`))

(event `MC_DeathSound`
  (params (Sound :type "SoundBase Object Reference") (Location :type "Vector Structure"))
  ;[1 0 0.4922] 敌人死亡事件
  (`GameplayStatics.PlaySoundAtLocation` Sound Location (struct) 1.0 1.0 0.0 null null null null))

(event `CL_RestartBehaviorTree`
  ;[1 0 0.2578] Restart Behavior Tree
  (`MovementComponent.StopMovementImmediately` (`self.CharacterMovement`))
  (`BrainComponent.StopLogic` (`AIController.BrainComponent` (`AIBlueprintHelperLibrary.GetAIController` self)) "")
  (bind _aicontroller (message `/Game/Blueprints/Interfaces/INT_AIController.GetAIControllerRef` (`AIBlueprintHelperLibrary.GetAIController` self)))
  (message `/Game/Blueprints/Interfaces/INT_AIController.RunAITree` _aicontroller))

(event `/Game/Blueprints/Interfaces/INT_EnemyBase.EnemyFade`
  (params (bFade :type Boolean))
  ;[0.8516 0 1] Fade
  (`self.SRV_EnemyFade` bFade))

(event `SRV_EnemyFade`
  (params (bFade :type Boolean))
  ;[0.8516 0 1] Fade
  (bind _output_get (set `self.Fade` bFade))
  (if _output_get
    (bind (_direction _fadealpha) (`Timeline|FadingEnemy` :!via `PlayFromStart` :!label _label_2)
      (:`Update`
        (set `self.EnemyFadeColor` (`KismetMathLibrary.LinearColorLerp` (struct :`R` 1.0 :`G` 1.0 :`B` 1.0 :`A` 1.0) (struct :`R` 1.0 :`G` 1.0 :`B` 1.0) _fadealpha)))
      (:`Finished`
        (if (not (`self.Fade`))
          (`/Game/Blueprints/Interfaces/INT_EnemyBase.Death` false)
          (`/Game/Blueprints/Interfaces/INT_EnemyBase.RestartBehaviorTree`))))
    (else
      (`CharacterMovementComponent.SetMovementMode` (`self.CharacterMovement`) "MOVE_Walking" 0)
      (goto _label_2 :!via `ReverseFromEnd`))))

(fn `GetEnemyRef`
  (returns (Enemy :type "/Game/Blueprints/Enemy/BP_EnemyBase Object Reference"))
  (return self))

(fn `OnRep_bIsMoving`
  (bind _sprite (`self.Sprite`))
  (bind (_idleanimation _moveanimation) (break `/Game/Blueprints/Structs/ST_EnemyInfo` (`self.EnemyInfo`)))
  (if true
    (`PaperFlipbookComponent.SetFlipbook` _sprite _moveanimation)
    (else
      (`PaperFlipbookComponent.SetFlipbook` _sprite _idleanimation))))

(fn `OnRep_EnemyFadeColor`
  (`PaperFlipbookComponent.SetSpriteColor` (`self.Sprite`) (`self.EnemyFadeColor`)))

(fn `OnRep_Is Death`
  (if (`self.Is Death`)
    (`/Game/Blueprints/Interfaces/INT_EnemyBase.SetMovementState` "NewEnumerator8")
    (`PrimitiveComponent.SetMaterial` (`self.Sprite`) 0 "/Paper2D/TranslucentUnlitSpriteMaterial.TranslucentUnlitSpriteMaterial")
    (else
      (`PrimitiveComponent.SetMaterial` (`self.Sprite`) 0 "/Paper2D/MaskedUnlitSpriteMaterial.MaskedUnlitSpriteMaterial"))))

(fn `OnRep_MovementState`
  (bind _sprite (`self.Sprite`))
  (bind ((`IdleAnimation_8_55CE9A484CB3BFA33390349E0EFA924D` _idleanimation) (`MoveAnimation_9_9E8CBA8C4270F95997717493DCDC2BCC` _moveanimation) (`DeathAnimation_10_037A5F184F154B36F86D40A0BFEBB10B` _deathanimation) (`HitAnimation_11_B358D2E249814CF6A9EB49AB01779131` _hitanimation)) (break `/Game/Blueprints/Structs/ST_EnemyInfo` (`self.EnemyInfo`)))
  (switch `/Game/Blueprints/Enums/E_MovementState` (`self.MovementState`)
    (:`NewEnumerator0`
      (`PaperFlipbookComponent.SetFlipbook` _sprite _idleanimation))
    (:`NewEnumerator1`
      (`PaperFlipbookComponent.SetFlipbook` _sprite _moveanimation))
    (:`NewEnumerator2`
      (`PaperFlipbookComponent.SetFlipbook` _sprite _moveanimation))
    (:`NewEnumerator9`
      (`PaperFlipbookComponent.SetFlipbook` _sprite _hitanimation))
    (:`NewEnumerator8`
      (`PaperFlipbookComponent.SetFlipbook` _sprite _deathanimation))))

(fn `OnRep_SpawnLocation`
  (`self.K2_SetActorLocation` (`self.SpawnLocation`)))

(fn `UserConstructionScript`
  (`parent.UserConstructionScript`))
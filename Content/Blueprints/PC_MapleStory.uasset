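; Player controller for a MapleStory game that handles character selection, pawn spawning and HUD updates.
; On BeginPlay it shows the cursor and character selection widget, and creates the main HUD without adding it to the viewport.
; Selection passes through an SRV event to a GameMode interface request, while a separate SpawnActor event spawns and possesses the pawn.
; Health bar and level updates reach the main HUD through CL events.
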(event `self.ReceiveBeginPlay`
  (`/Game/Blueprints/Interfaces/INT_PlayerController.ShowMainUIToViewport`))

(event `/Game/Blueprints/Interfaces/INT_PlayerController.ShowMainUIToViewport`
  ;[1 1 1] 添加UI到视口
  (`self.CL_ShowMainUIToViewport`))

(event `CL_ShowMainUIToViewport`
  ;[1 1 1] 添加UI到视口
  (set `self.bShowMouseCursor` true)
  (bind _returnvalue (`|CreateWidget` "/Game/Blueprints/Widgets/WBP_CharacterSelection.WBP_CharacterSelection_C"))
  (bind _output_get (set `self.CS_CharacterSelect` _returnvalue))
  (`UserWidget.AddToViewport` _output_get 0)
  (bind _returnvalue_2 (`|CreateWidget` "/Game/Blueprints/Widgets/WB_Main.WB_Main_C"))
  (set `self.WB_Main` _returnvalue_2))

(event `/Game/Blueprints/Interfaces/INT_PlayerController.SelectCharacter`
  (params (Player :type "Actor Class Reference") (SpawnLocation :type "Vector Structure"))
  ;[1 1 1] 选择角色
  (`self.SRV_SelectCharacter` Player SpawnLocation))

(event `SRV_SelectCharacter`
  (params (Player :type "Actor Class Reference") (SpawnLocation :type "Vector Structure"))
  ;[1 1 1] 选择角色
  (bind _gamemode (message `/Game/Blueprints/Interfaces/INT_GameMode.GameModeRef` (`GameplayStatics.GetGameMode`)))
  (message `/Game/Blueprints/Interfaces/INT_GameMode.RequestSpawnPlayer` _gamemode self Player SpawnLocation))

(event `/Game/Blueprints/Interfaces/INT_PlayerController.SpawnActor`
  (params (Player :type "Actor Class Reference") (SpawnTransform :type "Transform Structure"))
  (bind _returnvalue (`|SpawnActorFromClass` Player SpawnTransform "AdjustIfPossibleButAlwaysSpawn" "OverrideRootScale" null null))
  ;[1 1 1] 设置生成Actor的控制所有权
  (bind _player (message `/Game/Blueprints/Interfaces/INT_PlayerBase.PlayerRef` _returnvalue))
  (`self.Possess` _player))

(event `/Game/Blueprints/Interfaces/INT_PlayerController.UpdateHealthBar`
  (params (Health :type "Float (double-precision)") (EnemyName :type Name))
  ;[1 1 1] 更新血条
  (`self.CL_UpdateHealthBar` Health EnemyName))

(event `/Game/Blueprints/Interfaces/INT_PlayerController.UpdateLevelMsg`
  (params (PlayerInfo :type "/Game/Blueprints/Structs/ST_PlayerInfo Structure"))
  ;[1 1 1] 更新等级信息
  (`self.CL_UpdateLevelMsg` PlayerInfo))

(event `CL_UpdateHealthBar`
  (params (Percent :type "Float (single-precision)") (EnemyName :type Name))
  ;[1 1 1] 更新血条
  (`/Game/Blueprints/Widgets/WB_Main.UpdateHealth` (`self.WB_Main`) Percent EnemyName))

(event `CL_UpdateLevelMsg`
  (params (PlayerInfo :type "/Game/Blueprints/Structs/ST_PlayerInfo Structure"))
  ;[1 1 1] 更新等级信息
  (`/Game/Blueprints/Widgets/WB_Main.UpdateLevel` (`self.WB_Main`) PlayerInfo))

(fn `PlayerControllerRef`
  (returns (PlayerController :type "/Game/Blueprints/PC_MapleStory Object Reference"))
  (return self))

(fn `UserConstructionScript`)